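; BP_Pc_Lobby is the lobby player controller that owns the lobby UI and feeds it player names.
; On BeginPlay, only the local controller creates a WBP_Lobby widget, adds it to the viewport and stores the reference.
; AddPlayerToLobbyList reads the player name from a given controller's PlayerState and passes it as text to the widget's OnAddNewPLayer.
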(event `self.ReceiveBeginPlay`
  (if (`self.IsLocalController`)
    (bind _returnvalue (`|CreateWidget` "/Game/Blueprints/UI/WBP_Lobby.WBP_Lobby_C" self))
    (`UserWidget.AddToViewport` _returnvalue 0)
    (set `self.widgetRef` _returnvalue)))

(event `AddPlayerToLobbyList`
  (params (controller :type "Controller Object Reference"))
  (`/Game/Blueprints/UI/WBP_Lobby.OnAddNewPLayer` (`self.widgetRef`) (`KismetTextLibrary.Conv_StringToText` (`PlayerState.GetPlayerName` (`Controller.PlayerState` controller)))))

(fn `UserConstructionScript`)